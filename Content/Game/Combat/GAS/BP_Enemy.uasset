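; BP_Enemy is a combat enemy character that chases the player, attacks in melee range and shows a health widget.
; A health-change binding updates the widget with the normalized value.
; Tick drives simple AI without a behavior tree, issuing move orders or facing the player for a montage attack, with a random cooldown on completion.
; On death it ragdolls, calls EnemyDied and destroys itself after a delay.
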(event Custom|HandleHPChanged
  (params (NewValue :type Float%20%28single-precision%29) (MaxValue :type Float%20%28single-precision%29))
  (Default|SetHP (Variables|Default|GetHPWidget) (/ NewValue MaxValue)))

(event EventBeginPlay
  (bind _aswbp_enemy_health (Utilities|Casting|CastToWBP_EnemyHealth (UserInterface|GetUserWidgetObject (Variables|Default|GetHealthWidget))))
  (bind _output_get (Variables|Default|SetHPWidget _aswbp_enemy_health))
  (Default|SetHP _output_get (/ (Class|CombatCharacterBase|GetHealth) (Class|CombatCharacterBase|GetMaxHealth)))
  (EventDispatchers|BindEventtoOnHealthChanged (delegate Custom|HandleHPChanged)))

(event Collision|EventActorBeginOverlap
  (params (OtherActor :type Actor%20Object%20Reference)))

(event EventTick
  (params (DeltaSeconds :type Float%20%28single-precision%29))
  (bind _returnvalue (Game|GetPlayerCharacter 0))
  (bind _self self)
  (if (not (Variables|Default|GetbIsDead))
    (if (not (Variables|Default|GetbAttacking))
      (if (not (Class|AnimInstance|IsAnyMontagePlaying (Components|SkeletalMesh|GetAnimInstance (Variables|Character|GetMesh))))
        (if (Utilities|IsValid _returnvalue)
          (if (> (Transformation|GetDistanceTo _returnvalue) (Variables|Default|GetAttackRange))
            (if (Utilities|Enum|Equal(Enum) (Class|AIController|GetMoveStatus (AI|GetAIController _self)) "Idle")
              (AI|AIMoveTo _self "0, 0, 0" _returnvalue 1e+02 false))
            (else
              (Variables|Default|SetbAttacking true)
              (AI|Navigation|StopMovement (AI|GetAIController self))
              (Transformation|SetActorRotation (Math|Rotator|MakeRotator 0.0 0.0 (.Yaw (Math|Rotator|BreakRotator (Math|Rotator|FindLookatRotation (Transformation|GetActorLocation) (Transformation|GetActorLocation _returnvalue))))))
              (Animation|Montage|PlayMontage (Variables|Character|GetMesh) "/Game/Game/Enemy/AM_Enemy_Attack.AM_Enemy_Attack"
                (:OnCompleted
                  (Utilities|FlowControl|Delay (Math|Random|RandomFloatinRange 0.8 1.6)))
                (:OnInterrupted
                  _))
              (Variables|Default|SetbAttacking false))))))))

(event EventOnDeath
  (bind _mesh (Variables|Character|GetMesh))
  (Animation|StopAnimMontage 0)
  (AI|Navigation|StopMovement (AI|GetAIController self))
  (Collision|SetCollisionProfileName _mesh "Ragdoll" true :!class /Script/Engine.PrimitiveComponent)
  (Physics|SetSimulatePhysics _mesh true)
  (Collision|SetCollisionEnabled (Variables|Default|GetCapsuleComponent) "NoCollision")
  (Pawn|Components|CharacterMovement|DisableMovement (Variables|Character|GetCharacterMovement))
  (Default|CallEnemyDied)
  (Utilities|FlowControl|Delay 4.0)
  (Actor|DestroyActor))

(fn ConstructionScript)